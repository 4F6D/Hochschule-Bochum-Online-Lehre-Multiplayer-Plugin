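; Main menu player controller that shows and hides the main menu, create server and server browser widgets.
; BeginPlay shows the main menu through a ShowHideWidgets event, which acts only on the local controller.
; The show function creates each widget on first use, caches it and adds it to the viewport; the hide function removes it from its parent, keeping the cached reference.
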(event Custom|ShowHideWidgets
  (params (Widget :type E_MainMenuWidgets%20Enum :default "NewEnumerator0") (Show :type Boolean))
  (if (Pawn|IsLocalPlayerController)
    (if Show
      (CallFunction|FShowWidget Widget)
      (else
        (CallFunction|FHideWidget Widget)))))

(event EventBeginPlay
  (CallFunction|ShowHideWidgets "NewEnumerator0" true))

(fn ConstructionScript)

(fn FShowWidget
  (params (Widget :type E_MainMenuWidgets%20Enum :default "NewEnumerator0"))
  (switch Utilities|FlowControl|Switch|SwitchonE_MainMenuWidgets Widget
    (:NewEnumerator0
      (Variables|Default|GetWB_MainMenu
        (:then
          _)
        (:else
          (bind _returnvalue (UserInterface|CreateWidget "/Game/UI/MainMenu/WB_MainMenu.WB_MainMenu_C"))
          (bind _output_get (Variables|Default|SetWB_MainMenu _returnvalue))))
      (UserInterface|Viewport|AddtoViewport _output_get 0))
    (:NewEnumerator1
      (Variables|Default|GetWB_CreateServer
        (:then
          _)
        (:else
          (bind _returnvalue_2 (UserInterface|CreateWidget "/Game/UI/MainMenu/WB_CreateServer.WB_CreateServer_C"))
          (bind _output_get_2 (Variables|Default|SetWB_CreateServer _returnvalue_2))))
      (UserInterface|Viewport|AddtoViewport _output_get_2 0))
    (:NewEnumerator2
      (Variables|Default|GetServerBrowser
        (:then
          _)
        (:else
          (bind _returnvalue_3 (UserInterface|CreateWidget "/Game/UI/MainMenu/WB_ServerBrowser.WB_ServerBrowser_C"))
          (bind _output_get_3 (Variables|Default|SetServerBrowser _returnvalue_3))))
      (UserInterface|Viewport|AddtoViewport _output_get_3 0))))

(fn FHideWidget
  (params (Widget :type E_MainMenuWidgets%20Enum :default "NewEnumerator0"))
  (switch Utilities|FlowControl|Switch|SwitchonE_MainMenuWidgets Widget
    (:NewEnumerator0
      (bind _wb_mainmenu (Variables|Default|GetWB_MainMenu)
        (:then
          (Widget|RemovefromParent _wb_mainmenu))
        (:else)))
    (:NewEnumerator1
      (bind _wb_createserver (Variables|Default|GetWB_CreateServer)
        (:then
          (Widget|RemovefromParent _wb_createserver))
        (:else)))
    (:NewEnumerator2
      (bind _serverbrowser (Variables|Default|GetServerBrowser)
        (:then
          (Widget|RemovefromParent _serverbrowser))
        (:else)))))

(fn GetPlayerControllerRef
  (return self))